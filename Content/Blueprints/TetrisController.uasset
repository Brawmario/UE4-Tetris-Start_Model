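; TetrisController is the input handler for a Tetris game, passing key presses to the TetrisGameMode.
; It casts and caches the game mode on BeginPlay.
; Left, Right and Down move the piece by a fixed grid step in world X and Z, Up rotates it, and SpaceBar creates a piece.
; All movement, rotation and spawning logic is delegated to the game mode.
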(event `Key|Left`
  (params (Key :type "Key Structure"))
  (:`Pressed`
    (`/Game/Blueprints/TetrisGameMode.MovePiece` (`self.GameMode`) 101.0 0.0 0.0)))

(event `Key|Right`
  (params (Key :type "Key Structure"))
  (:`Pressed`
    (`/Game/Blueprints/TetrisGameMode.MovePiece` (`self.GameMode`) -101.0 0.0 0.0)))

(event `Key|Up`
  (params (Key :type "Key Structure"))
  (:`Pressed`
    (`/Game/Blueprints/TetrisGameMode.RotatePiece` (`self.GameMode`))))

(event `Key|Down`
  (params (Key :type "Key Structure"))
  (:`Pressed`
    (`/Game/Blueprints/TetrisGameMode.MovePiece` (`self.GameMode`) 0.0 0.0 -101.0)))

(event `self.ReceiveBeginPlay`
  (bind _astetris_game_mode (cast `/Game/Blueprints/TetrisGameMode` (`GameplayStatics.GetGameMode`)))
  (set `self.GameMode` _astetris_game_mode))

(event `Key|SpaceBar`
  (params (Key :type "Key Structure"))
  (:`Pressed`
    (`/Game/Blueprints/TetrisGameMode.CreatePiece` (`self.GameMode`))))

(fn `UserConstructionScript`)